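; Moving platform actor with a TileMap component that travels between its start location and an EndPoint.
; On BeginPlay it records the TileMap's world location and converts EndPoint from relative to world space.
; The Alpha timeline, with looping set by a variable and play rate derived from Duration, lerps the actor there and back without sweeping.
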(event `self.ReceiveBeginPlay`
  (bind _alpha (`self.Alpha`))
  (bind _returnvalue (`SceneComponent.K2_GetComponentToWorld` (`self.TileMap`)))
  (set `self.StartPoint` (.location _returnvalue))
  ;[1 1 1] EndPoint is a relative position, we need the world one
  (set `self.EndPoint` (`KismetMathLibrary.TransformLocation` _returnvalue (`self.EndPoint`)))
  ;[1 1 1] Move the actor to EndPoint and back
  (`TimelineComponent.SetLooping` _alpha (`self.Looping`))
  (`TimelineComponent.SetPlayRate` _alpha (/ 1.0 (`self.Duration`)))
  (bind (_direction _alpha_2) (`Timeline|Alpha`)
    (:`Update`
      (`self.K2_SetActorLocation` (`KismetMathLibrary.VLerp` (`self.StartPoint`) (`self.EndPoint`) _alpha_2)))))

(fn `UserConstructionScript`)