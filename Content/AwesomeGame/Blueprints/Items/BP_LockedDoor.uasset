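; BP_LockedDoor is a door actor that checks whether the player character holds a key.
; Its Collision component enables input from player controller 0 while a MyAwesomeGameCharacter overlaps it and disables it when the overlap ends.
; Pressing Action reads the character's HasKey flag and only prints an open or locked message; no door opening is implemented.
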(event `self.ReceiveBeginPlay`)

(event `self.ReceiveActorBeginOverlap`
  (params (OtherActor :type "Actor Object Reference")))

(event `self.ReceiveTick`
  (params (DeltaSeconds :type "Float (single-precision)")))

(event `self.Collision.OnComponentBeginOverlap`
  (params (OtherActor :type "Actor Object Reference") (OtherComp :type "PrimitiveComponent Object Reference") (OtherBodyIndex :type Integer) (bFromSweep :type Boolean) (SweepResult :type "HitResult Structure (by ref)"))
  (cast `/Game/AwesomeGame/Blueprints/MyAwesomeGameCharacter` OtherActor)
  (`self.EnableInput` (`GameplayStatics.GetPlayerController` 0)))

(event `self.Collision.OnComponentEndOverlap`
  (params (OtherActor :type "Actor Object Reference") (OtherComp :type "PrimitiveComponent Object Reference") (OtherBodyIndex :type Integer))
  (cast `/Game/AwesomeGame/Blueprints/MyAwesomeGameCharacter` OtherActor)
  (`self.DisableInput` (`GameplayStatics.GetPlayerController` 0)))

(event `InputAction|Action`
  (:`Pressed`
    (bind _asmy_awesome_game_character (cast `/Game/AwesomeGame/Blueprints/MyAwesomeGameCharacter` (`GameplayStatics.GetPlayerCharacter` 0)))
    (if (`/Game/AwesomeGame/Blueprints/MyAwesomeGameCharacter.HasKey` _asmy_awesome_game_character)
      (`KismetSystemLibrary.PrintString` "OPEN")
      (else
        (`KismetSystemLibrary.PrintString` "locked")))))

(fn `UserConstructionScript`)