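; A 2D player character Blueprint that blinks its sprite as feedback when it takes damage.
; AnyDamage starts a looping timer on Blink, which toggles sprite visibility, then clears it after a short delay and forces the sprite visible.
; Pressing F applies a small amount of damage to the character itself, triggering the blink.
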(event `self.ReceiveActorBeginOverlap`
  (params (OtherActor :type "Actor Object Reference")))

(event `self.ReceiveTick`
  (params (DeltaSeconds :type "Float (single-precision)")))

(event `Key|F`
  (:`Pressed`
    (`GameplayStatics.ApplyDamage` self 0.1)))

(event `self.ReceiveAnyDamage`
  (params (Damage :type "Float (single-precision)") (DamageType :type "DamageType Object Reference") (InstigatedBy :type "Controller Object Reference") (DamageCauser :type "Actor Object Reference"))
  (`KismetSystemLibrary.K2_SetTimer` null "Blink" 0.1 true)
  (`KismetSystemLibrary.Delay` 1.3)
  (`KismetSystemLibrary.K2_ClearTimer` null "Blink")
  (`SceneComponent.SetVisibility` (`self.Sprite`) true false))

(event `Blink`
  (`SceneComponent.ToggleVisibility` (`self.Sprite`) false))

(fn `UserConstructionScript`)