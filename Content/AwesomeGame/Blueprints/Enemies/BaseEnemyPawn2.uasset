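; Base enemy pawn with Mario-style stomp combat against MyAwesomeGameCharacter.
; On a collision hit by that character, an impact normal pointing down within a tolerance counts as a top hit and damages the enemy; any other hit damages the hero.
; AnyDamage subtracts from Life, destroying the pawn at zero or below and otherwise printing a debug message.
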(event `self.Collision.OnComponentHit`
  (params (OtherActor :type "Actor Object Reference") (OtherComp :type "PrimitiveComponent Object Reference") (NormalImpulse :type "Vector Structure") (Hit :type "HitResult Structure (by ref)"))
  (bind _asmy_awesome_game_character (cast `/Game/AwesomeGame/Blueprints/MyAwesomeGameCharacter` OtherActor))
  (if (== Hit_ImpactNormal (`KismetMathLibrary.MakeVector` (.x Hit_ImpactNormal) (.y Hit_ImpactNormal) -1.0) :`ErrorTolerance` 0.1)
    (`GameplayStatics.ApplyDamage` self 0.1 null _asmy_awesome_game_character) ; Damage the monster when hit on top
    (else
      (`GameplayStatics.ApplyDamage` _asmy_awesome_game_character 0.1 null self) ; Damage the hero
    )))

(event `self.ReceiveAnyDamage`
  (params (Damage :type "Float (single-precision)") (DamageType :type "DamageType Object Reference") (InstigatedBy :type "Controller Object Reference") (DamageCauser :type "Actor Object Reference"))
  (bind _output_get (set `self.Life` (- (`self.Life`) Damage)))
  (if (<= _output_get 0.0)
    (`self.K2_DestroyActor`)
    (else
      (`KismetSystemLibrary.PrintString` "Takes damage"))))

(fn `UserConstructionScript`)