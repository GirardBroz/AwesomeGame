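; A moving platform actor for level structure that travels between its starting location and an end point, optionally looping.
; On BeginPlay it converts the relative EndPoint to world space and plays a timeline with its rate scaled by Duration.
; The timeline alpha is remapped onto the Movement curve's time range, so any curve shapes the interpolation.
; Each update sets the location without sweeping.
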(event `self.ReceiveBeginPlay`
  (bind _returnvalue (`self.GetTransform`))
  (bind _movement (`self.Movement`))
  (bind _timedrivingtimeline (`self.TimeDrivingTimeline`))
  (bind (_mintime _maxtime) (`CurveBase.GetTimeRange` _movement))
  (set `self.StartPoint` (.location _returnvalue))
  ;[1 1 1] EndPoint is a relative position, we need the world one
  (set `self.EndPoint` (`KismetMathLibrary.TransformLocation` _returnvalue (`self.EndPoint`)))
  ;[1 1 1] Move the actor to EndPoint and back
  (`TimelineComponent.SetLooping` _timedrivingtimeline (`self.Looping`))
  (`TimelineComponent.SetPlayRate` _timedrivingtimeline (/ 1.0 (`self.Duration`)))
  (bind (_direction _timealpha) (`Timeline|TimeDrivingTimeline`)
    (:`Update`
      (`self.K2_SetActorLocation` (`KismetMathLibrary.VLerp` (`self.StartPoint`) (`self.EndPoint`) (`CurveFloat.GetFloatValue` _movement (`KismetMathLibrary.Lerp` _mintime _maxtime _timealpha)))))))

(fn `UserConstructionScript`)